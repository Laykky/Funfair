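; BP_AttractionTrigger is a trigger volume that tracks whether the player is inside an attraction's play area.
; When a Player-tagged BP_ThirdPersonCharacter enters the TriggerBox, it stores the character and calls StartPlaying; exiting calls StopPlaying.
; These functions only toggle the Playing flag.
; Nodes for contextual camera blending and the ChambouleTout HUD are disconnected, so entering changes neither view nor UI, despite the event comments.
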(event `self.TriggerBox.OnComponentBeginOverlap`
  (params (OverlappedComponent :type "PrimitiveComponent Object Reference") (OtherActor :type "Actor Object Reference") (OtherComp :type "PrimitiveComponent Object Reference") (OtherBodyIndex :type Integer) (bFromSweep :type Boolean) (SweepResult :type "HitResult Structure (by ref)"))
  ;[0.349 1 0.6536] Si l'acteur à le tag player alors en rentrant dans la la triggerbox mettre la caméra "contextuelle"
  (if (`self.ActorHasTag` OtherActor "Player")
    (bind _asbp_third_person_character (cast `/Game/ThirdPerson/Blueprints/BP_ThirdPersonCharacter` OtherActor))
    (set `self.As BP Third Person Character` _asbp_third_person_character)
    (`self.StartPlaying`)))

(event `self.TriggerBox.OnComponentEndOverlap`
  (params (OverlappedComponent :type "PrimitiveComponent Object Reference") (OtherActor :type "Actor Object Reference") (OtherComp :type "PrimitiveComponent Object Reference") (OtherBodyIndex :type Integer))
  ;[0.2602 1 0.6012] Si l'acteur à le tag player alors en sortant de la triggerbox remettre la caméra de base
  (if (`self.ActorHasTag` OtherActor "Player")
    (cast `/Game/ThirdPerson/Blueprints/BP_ThirdPersonCharacter` OtherActor)
    (`self.StopPlaying`)))

(fn `StartPlaying`
  (set `self.Playing` true))

(fn `StopPlaying`
  (set `self.Playing` false))

(fn `UserConstructionScript`)