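; Chamboule-tout (knock-down) minigame Blueprint that extends a parent's start/stop logic with shooting, a dedicated camera and a crosshair HUD.
; StartPlaying enables the character's shooting, switches the view to the triggered camera's owner and creates the HUD.
; StopPlaying disables shooting, returns the view to the pawn and removes the HUD.
; While Playing, Tick moves the crosshair to the mouse position.
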(event `self.ReceiveTick`
  (params (DeltaSeconds :type "Float (single-precision)"))
  (bind (_locationx _locationy) (`PlayerController.GetMousePosition` (`GameplayStatics.GetPlayerController` 0)))
  (if (`self.Playing`)
    (`CanvasPanelSlot.SetPosition` (`WidgetLayoutLibrary.SlotAsCanvasSlot` (`/Game/BluePrints/WB_ChambouleTout_HUD.Crosshair` (`self.ChambouleToutHUD`))) (`SlateBlueprintLibrary.ScreenToViewport` (`KismetMathLibrary.MakeVector2D` _locationx _locationy)))))

(fn `StartPlaying`
  (`parent.StartPlaying`)
  (set `/Game/ThirdPerson/Blueprints/BP_ThirdPersonCharacter.CanShoot` true (`self.As BP Third Person Character`))
  (`PlayerController.SetViewTargetWithBlend` (`GameplayStatics.GetPlayerController` 0) (`ActorComponent.GetOwner` (`self.TriggeredCamera`)) 0.0 "VTBlend_Linear" 0.0 false)
  (bind _returnvalue (`|CreateWidget` "/Game/BluePrints/WB_ChambouleTout_HUD.WB_ChambouleTout_HUD_C" (`GameplayStatics.GetPlayerController` 0)))
  (`UserWidget.AddToViewport` _returnvalue 0))

(fn `StopPlaying`
  (bind _returnvalue (`GameplayStatics.GetPlayerController` 0))
  (`parent.StopPlaying`)
  (set `/Game/ThirdPerson/Blueprints/BP_ThirdPersonCharacter.CanShoot` false (`self.As BP Third Person Character`))
  (`PlayerController.SetViewTargetWithBlend` _returnvalue (`Controller.K2_GetPawn` _returnvalue) 0.0 "VTBlend_Linear" 0.0 false)
  (`Widget.RemoveFromParent` (`self.ChambouleToutHUD`)))

(fn `UserConstructionScript`
  (`parent.UserConstructionScript`))