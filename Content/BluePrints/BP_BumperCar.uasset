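; BP_BumperCar is a bumper car driven through Enhanced Input actions on a static mesh.
; AI_CarMove adds physics force along the mesh's forward vector, while AI_CarTurn sets world yaw directly from TurnSpeed, zeroing pitch and roll.
; Pressing E calls Possess on player controller 0, with no target pawn supplied.
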(event `EnhancedInput|/Game/BluePrints/AI_CarMove`
  (params (ActionValue :type "Float (double-precision)") (ElapsedSeconds :type "Float (double-precision)") (TriggeredSeconds :type "Float (double-precision)") (InputAction :type "InputAction Object Reference" :default "/Game/BluePrints/AI_CarMove.AI_CarMove"))
  (bind _staticmesh (`self.StaticMesh`))
  (:`Triggered`
    (`PrimitiveComponent.AddForce` _staticmesh (* (`SceneComponent.GetForwardVector` _staticmesh) (`self.MoveForce`) ActionValue) "None" false)))

(event `EnhancedInput|/Game/BluePrints/AI_CarTurn`
  (params (ActionValue :type "Float (double-precision)") (ElapsedSeconds :type "Float (double-precision)") (TriggeredSeconds :type "Float (double-precision)") (InputAction :type "InputAction Object Reference" :default "/Game/BluePrints/AI_CarTurn.AI_CarTurn"))
  (bind _staticmesh (`self.StaticMesh`))
  (bind (_returnvalue_roll _returnvalue_pitch _returnvalue_yaw) (`KismetMathLibrary.BreakRotator` (`SceneComponent.K2_GetComponentRotation` _staticmesh)))
  (:`Triggered`
    (`SceneComponent.K2_SetWorldRotation` _staticmesh (`KismetMathLibrary.MakeRotator` 0.0 0.0 (+ _returnvalue_yaw (* ActionValue (`self.TurnSpeed`)))) false false)))

(event `Key|E`
  (params (Key :type "Key Structure"))
  (:`Pressed`
    (`Controller.Possess` (`GameplayStatics.GetPlayerController` 0) null)))

(fn `UserConstructionScript`)