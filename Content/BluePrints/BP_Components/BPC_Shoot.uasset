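; Actor component that fires physics-driven BP_Ball projectiles from its owner, with force scaled by charge time.
; Shoot lerps between min and max force by ShootTime, spawns the ball ahead of and slightly above the owner, then applies an impulse along player 0's deprojected mouse direction.
; GetShootTimeNormalized multiplies ShootForce by MaxForce, despite its name.
; The EventGraph holds an unconnected earlier forward-arc version that never runs.
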(event `Key|LeftMouseButton`
  (params (Key :type "Key Structure"))
  ;[0.386 0.1536 1] On Left Click faire spawn une balle avec une impulsion PLUS UTILE
)

(fn `GetShootTimeNormalized`
  (returns (NormalizedShootForce :type "Float (double-precision)"))
  (return (* (`self.ShootForce`) (`self.MaxForce`))))

(fn `Shoot`
  (params (ShootTime :type "Float (double-precision)"))
  (bind _returnvalue (`GameplayStatics.GetPlayerController` 0))
  (bind _returnvalue_2 (`self.GetOwner`))
  (bind (_locationx _locationy) (`PlayerController.GetMousePosition` _returnvalue))
  (set `self.ShootForce` (`KismetMathLibrary.Lerp` (`self.MinForce`) (`self.MaxForce`) (/ ShootTime (`self.MaxShootTime`))))
  (bind _returnvalue_3 (`|SpawnActorFromClass` "/Game/BluePrints/BP_Ball.BP_Ball_C" (`KismetMathLibrary.MakeTransform` (+ (`Actor.K2_GetActorLocation` _returnvalue_2) (* (`KismetMathLibrary.MakeVector` (.x (`Actor.GetActorForwardVector` _returnvalue_2)) (.y (`Actor.GetActorForwardVector` _returnvalue_2)) (+ (.z (`Actor.GetActorForwardVector` _returnvalue_2)) 0.2)) 100.0))) "Undefined" "MultiplyWithRoot" null null))
  (bind _sphere (`/Game/BluePrints/BP_Ball.Sphere` _returnvalue_3))
  (`PrimitiveComponent.SetSimulatePhysics` _sphere true)
  (`PrimitiveComponent.SetEnableGravity` _sphere true)
  (`PrimitiveComponent.SetLinearDamping` _sphere 0.2)
  (`PrimitiveComponent.AddImpulse` _sphere (* (`.WorldDirection` (`GameplayStatics.DeprojectScreenToWorld` _returnvalue (`KismetMathLibrary.MakeVector2D` _locationx _locationy))) (`self.ShootForce`)) "None" false))