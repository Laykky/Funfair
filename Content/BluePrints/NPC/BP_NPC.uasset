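; BP_NPC is a wandering NPC that moves endlessly between randomly chosen BP_TargetPoint actors in the level.
; BeginPlay caches the target points, and the recursive Move event retries on Creation or Destruction types and calls AIMoveTo on Regular.
; Move runs again whether the move succeeds or fails.
; The NavType check draws its own random point, so it can differ from the stored destination.
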(event `self.ReceiveBeginPlay`
  (bind _outactors (`GameplayStatics.GetAllActorsOfClass` "/Game/BluePrints/BP_TargetPoint.BP_TargetPoint_C"))
  (set `self.TargetPoints` _outactors)
  (`self.Move`))

(event `Move`
  (bind _outitem (`KismetArrayLibrary.Array_Random` (`self.TargetPoints`)))
  (set `self.RandomTP` _outitem)
  (switch `/Game/BluePrints/Enumerator/E_NavTargetPointType` (`/Game/BluePrints/BP_TargetPoint.NavType` _outitem)
    (:`NewEnumerator0`
      (`self.Move`))
    (:`NewEnumerator1`
      (`self.Move`))
    (:`NewEnumerator2`
      (`|AIMoveTo` self (`self.K2_GetActorLocation` (`self.RandomTP`)) null
        (:`OnSuccess`
          _)
        (:`OnFail`
          _))
      (`self.Move`))))

(fn `UserConstructionScript`)